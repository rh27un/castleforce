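; HexMetrics is an actor that computes the basic dimensions of a hexagon from its OuterRadius.
; On BeginPlay it derives InnerRadius using the √3/2 ratio, then fills the Corners array with six local offsets in the XY plane, starting at the +Y vertex.
; The values are set only at runtime, as the Construction Script is empty.
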(event `self.ReceiveBeginPlay`
  (set `self.Inner Radius` (* (`self.Outer Radius`) 0.866025))
  (set `self.Corners` (`|MakeArray` (`KismetMathLibrary.MakeVector` 0.0 (`self.Outer Radius`)) (`KismetMathLibrary.MakeVector` (`self.Inner Radius`) (* (`self.Outer Radius`) 0.5)) (`KismetMathLibrary.MakeVector` (`self.Inner Radius`) (* (`self.Outer Radius`) -0.5)) (`KismetMathLibrary.MakeVector` 0.0 (- 0.0 (`self.Outer Radius`))) (`KismetMathLibrary.MakeVector` (- 0.0 (`self.Inner Radius`)) (* (`self.Outer Radius`) -0.5)) (`KismetMathLibrary.MakeVector` (- 0.0 (`self.Inner Radius`)) (* (`self.Outer Radius`) 0.5)))))

(fn `UserConstructionScript`)