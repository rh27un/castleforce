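; HexTile is a clickable hexagonal tile actor that builds its own mesh at runtime.
; On BeginPlay it finds the HexMetrics actor and creates a procedural mesh section with collision from that actor's corner vertices and its own triangle list, then applies a base material.
; Clicking the mesh prints a debug message and switches the material to blue.
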(event `self.ReceiveBeginPlay`
  (bind _proceduralmesh (`self.ProceduralMesh`))
  (bind _outactors (`GameplayStatics.GetAllActorsOfClass` "/Game/Blueprints/HexMetrics.HexMetrics_C"))
  (set `self.Metrics` (`|GetArrayItem` _outactors))
  (`ProceduralMeshComponent.CreateMeshSection_LinearColor` :`self` (`self.ProceduralMesh`) :`Vertices` (`/Game/Blueprints/HexMetrics.Corners` (`self.Metrics`)) :`Triangles` (`self.Triangles`) :`bCreateCollision` true)
  (`PrimitiveComponent.SetMaterial` _proceduralmesh 0 "/Game/Puzzle/Meshes/BaseMaterial.BaseMaterial")
  (`PrimitiveComponent.SetCollisionEnabled` _proceduralmesh "QueryAndPhysics"))

(event `self.ProceduralMesh.OnClicked`
  (params (TouchedComponent :type "PrimitiveComponent Object Reference") (ButtonPressed :type "Key Structure"))
  (`KismetSystemLibrary.PrintString` "Hello")
  (`PrimitiveComponent.SetMaterial` (`self.ProceduralMesh`) 0 "/Game/Puzzle/Meshes/BlueMaterial.BlueMaterial"))

(fn `UserConstructionScript`)